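; BP_Lava is a lava hazard actor that burns the third-person player character while it overlaps.
; Begin overlap stores the character and sets a Burn flag, which any actor's end overlap clears.
; While Burn is set, Tick spawns randomly scaled burning effects near the character's feet and calls BurningDamage.
; Delay nodes throttle both the spawning and the repeated one-point Health loss, despite per-frame calls.
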(event `self.ReceiveTick`
  (params (DeltaSeconds :type "Float (single-precision)"))
  (bind _returnvalue (`KismetMathLibrary.RandomFloatInRange` 0.5 1.0))
  (bind (_returnvalue_x _returnvalue_y _returnvalue_z) (`KismetMathLibrary.BreakVector` (`self.K2_GetActorLocation` (`self.As BP Third Person Character_0`))))
  ; Calls damage function and displays burnign effect.
  (if (`self.Burn`)
    (`self.BurningDamage`)
    (`KismetSystemLibrary.Delay` 0.05)
    (`|SpawnActorFromClass` "/Game/Objects/BP_BurningEffect.BP_BurningEffect_C" (`KismetMathLibrary.MakeTransform` (`KismetMathLibrary.MakeVector` _returnvalue_x _returnvalue_y (+ _returnvalue_z -50.0)) (struct) (`KismetMathLibrary.MakeVector` _returnvalue _returnvalue _returnvalue)) "Undefined" "MultiplyWithRoot" null null)))

(event `BurningDamage`
  ; Damages player
  (if (`self.Burn`)
    (set `self.EffectShow` true)
    (`KismetSystemLibrary.Delay` 0.4)
    (`/Engine/EditorBlueprintResources/StandardMacros.DecrementInt` (`/Game/ThirdPerson/Blueprints/BP_ThirdPersonCharacter.Health` (`self.As BP Third Person Character_0`))
      (:`  `
        (set `self.EffectShow` false)))))

(event `self.ReceiveActorBeginOverlap`
  (params (OtherActor :type "Actor Object Reference"))
  ; Controls when to damage player
  (bind _asbp_third_person_character (cast `/Game/ThirdPerson/Blueprints/BP_ThirdPersonCharacter` OtherActor))
  (set `self.As BP Third Person Character_0` _asbp_third_person_character)
  (set `self.Burn` true))

(event `self.ReceiveActorEndOverlap`
  (params (OtherActor :type "Actor Object Reference"))
  ; Controls when to damage player
  (set `self.Burn` false))

(fn `UserConstructionScript`)