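; BP_SaveStation is a checkpoint actor that sets the player's respawn location when BP_ThirdPersonCharacter overlaps it.
; On overlap it writes its Box component's world location into the character's SpawnPoint, skipping this if that point is already stored.
; A newly set checkpoint also spawns a BP_RespawnScan actor at the Cube component's location and prints a debug string.
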(event `self.ReceiveActorBeginOverlap`
  (params (OtherActor :type "Actor Object Reference"))
  (bind _returnvalue (`SceneComponent.K2_GetComponentLocation` (`self.Box`)))
  (bind _asbp_third_person_character (cast `/Game/ThirdPerson/Blueprints/BP_ThirdPersonCharacter` OtherActor))
  (if (not (== (`/Game/ThirdPerson/Blueprints/BP_ThirdPersonCharacter.SpawnPoint` _asbp_third_person_character) _returnvalue))
    (set `/Game/ThirdPerson/Blueprints/BP_ThirdPersonCharacter.SpawnPoint` _returnvalue _asbp_third_person_character)
    (`|SpawnActorFromClass` "/Game/Objects/BP_RespawnScan.BP_RespawnScan_C" (`KismetMathLibrary.MakeTransform` (`SceneComponent.K2_GetComponentLocation` (`self.Cube`))) "Undefined" "MultiplyWithRoot" null null)
    (`KismetSystemLibrary.PrintString` "Hello")))

(fn `UserConstructionScript`)