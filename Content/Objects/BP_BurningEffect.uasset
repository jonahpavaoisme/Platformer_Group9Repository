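; BP_BurningEffect is a drifting actor, likely a burning particle or ember effect, that rises upward after spawning.
; BeginPlay picks a random horizontal velocity and a random rotation on all axes.
; Tick moves it by that velocity each frame without sweeping, damping the horizontal speed and steadily increasing upward speed, so the motion is frame-rate dependent.
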(event `self.ReceiveBeginPlay`
  (set `self.Speeds` (`KismetMathLibrary.MakeVector` (`KismetMathLibrary.RandomFloatInRange` -5.0 5.0) (`KismetMathLibrary.RandomFloatInRange` -5.0 5.0)))
  (`self.K2_SetActorRotation` (`KismetMathLibrary.MakeRotator` (`KismetMathLibrary.RandomFloatInRange` 0.0 360.0) (`KismetMathLibrary.RandomFloatInRange` 0.0 360.0) (`KismetMathLibrary.RandomFloatInRange` 0.0 360.0))))

(event `self.ReceiveTick`
  (params (DeltaSeconds :type "Float (single-precision)"))
  (bind (_speeds_x _speeds_y _speeds_z) (`KismetMathLibrary.BreakVector` (`self.Speeds`)))
  (`self.K2_AddActorWorldOffset` (`self.Speeds`))
  (set `self.Speeds` (`KismetMathLibrary.MakeVector` (* _speeds_x 0.95) (* _speeds_y 0.95) (+ _speeds_z 1.0))))

(fn `UserConstructionScript`)